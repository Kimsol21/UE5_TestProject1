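; BP_FlyingPlayer is a flying player actor that currently implements only steering from the Turn input axis.
; Each axis update eases the SMBody mesh's roll toward an input-scaled bank angle with a fixed-alpha lerp, while yawing the whole actor in world space.
; Both rotations derive from TurnRate and world delta time, keeping the visual banking on the mesh separate from the actor's heading.
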(event `InputAxis|Turn`
  (params (AxisValue :type "Float (single-precision)"))
  (bind _returnvalue (* (`self.TurnRate`) (`GameplayStatics.GetWorldDeltaSeconds`) AxisValue))
  (bind (_relativerotation_roll _relativerotation_pitch) (`KismetMathLibrary.BreakRotator` (`SceneComponent.RelativeRotation` (`self.SM_Body`))))
  (bind _output_get (set `self.TargetRollRotation` (* _returnvalue 20.0)))
  (`SceneComponent.K2_SetRelativeRotation` (`self.SM_Body`) (`KismetMathLibrary.MakeRotator` (`KismetMathLibrary.Lerp` _relativerotation_roll _output_get 0.2) _relativerotation_pitch) false false)
  (`self.K2_AddActorWorldRotation` (`KismetMathLibrary.MakeRotator` 0.0 0.0 (* _returnvalue 0.5))))

(fn `UserConstructionScript`
  (`parent.UserConstructionScript`))