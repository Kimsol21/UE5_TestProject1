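; Player actor for a tile-grid game, tracking grid position, HP and gold, with HP set to max on BeginPlay.
; PositionChanged steps along one axis within map bounds, snaps the actor to 100-unit cells and returns that tile's index, monster flag and gold from the supplied flattened TileMap.
; HPChanged applies a clamped change and reports when HP reaches zero, while SetPlayerGold updates gold by addition.
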(event `self.ReceiveBeginPlay`
  (set `self.CurrentHP` (`self.MaxHP`)))

(fn `HPChanged`
  (params (ChangedValue :type Integer))
  (returns (bIsPlayerDead :type Boolean))
  (bind _output_get (set `self.CurrentHP` (`KismetMathLibrary.Clamp` (+ (`self.CurrentHP`) ChangedValue) 0 (`self.MaxHP`))))
  (return (== _output_get 0)))

(fn `PositionChanged`
  (params (bIsFrontDirection :type Boolean) (Position :type Integer) (MapSizeX :type Integer) (MapSizeY :type Integer) (TileMap :type "Array of /Game/My/Structures/TileInfo Structure"))
  (returns (bIsMonsterExist :type Boolean) (Gold :type Integer) (PlayerTileIndex :type Integer))
  (bind (_returnvalue_x _returnvalue_y _returnvalue_z) (`KismetMathLibrary.BreakVector` (`self.K2_GetActorLocation`)))
  (bind _returnvalue (+ (* (`self.XPos`) MapSizeY) (`self.YPos`)))
  (bind (_output_xpos _output_ypos _output_bexistmonster _output_gold) (break `/Game/My/Structures/TileInfo` (`|GetArrayItem` TileMap _returnvalue)))
  (`|ExecutionSequence`
    (:`then_0`
      (if bIsFrontDirection
        (set `self.XPos` (`KismetMathLibrary.Clamp` (+ (`self.XPos`) Position) 0 MapSizeX))
        (else
          (set `self.YPos` (`KismetMathLibrary.Clamp` (+ (`self.YPos`) Position) 0 MapSizeY))))
      (`self.K2_SetActorLocation` (`KismetMathLibrary.MakeVector` (`KismetMathLibrary.Conv_IntToDouble` (* (`self.XPos`) 100)) (`KismetMathLibrary.Conv_IntToDouble` (* (`self.YPos`) 100)) _returnvalue_z)))
    (:`then_1`
      (return _output_bexistmonster _output_gold _returnvalue))))

(fn `SetPlayerGold`
  (params (Gold :type Integer))
  (set `self.Gold` (+ (`self.Gold`) Gold)))

(fn `UserConstructionScript`)